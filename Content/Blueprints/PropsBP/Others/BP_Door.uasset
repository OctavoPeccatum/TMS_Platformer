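; BP_Door is an interactable door that swings open or shut when Interact fires while the third-person character is nearby.
; The Trigger overlap shows or removes an interact prompt widget and opens or closes a Gate that permits interaction.
; Interact briefly flags the prompt as pressed, then lerps the mesh's yaw using one timeline to open and another, reversed, to close.
; IsDoorClosed selects the direction and updates when the timeline finishes.
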(event OnComponentBeginOverlap(Trigger)
  (params (OverlappedComponent :type Primitive%20Component%20Object%20Reference) (OtherActor :type Actor%20Object%20Reference) (OtherComp :type Primitive%20Component%20Object%20Reference) (OtherBodyIndex :type Integer) (bFromSweep :type Boolean) (SweepResult :type Hit%20Result%20Structure%20%28by%20ref%29))
  (Utilities|Casting|CastToBP_ThirdPersonCharacter OtherActor)
  (bind _returnvalue (UserInterface|CreateWidget "/Game/Home_Platformer/HUD/Widgets/Interact_Promt_Widget.Interact_Promt_Widget_C"))
  (bind _output_get (Variables|Default|SetWidgetInteract _returnvalue))
  (UserInterface|Viewport|AddtoViewport _output_get 0)
  (Utilities|FlowControl|Gate true) ; enters at Open
)

(event OnComponentEndOverlap(Trigger)
  (params (OverlappedComponent :type Primitive%20Component%20Object%20Reference) (OtherActor :type Actor%20Object%20Reference) (OtherComp :type Primitive%20Component%20Object%20Reference) (OtherBodyIndex :type Integer))
  (Utilities|Casting|CastToBP_ThirdPersonCharacter OtherActor)
  (Widget|RemovefromParent (Variables|Default|GetWidgetInteract))
  (Utilities|FlowControl|Gate true) ; enters at Close
)

(event EventInteract
  (Variables|Default|SetIs%20Looking%20At%20Door? true)
  (Variables|/Game/Home_Platformer/HUD/Widgets/Interact_Promt_Widget.Interact_Promt_Widget_C|SetIs%20Pressed? (Variables|Default|GetWidgetInteract) true)
  (Utilities|FlowControl|Delay 0.2)
  (Variables|/Game/Home_Platformer/HUD/Widgets/Interact_Promt_Widget.Interact_Promt_Widget_C|SetIs%20Pressed? (Variables|Default|GetWidgetInteract) false)
  (if (Variables|Default|GetIs%20Looking%20At%20Door?)
    (Variables|Default|SetIs%20Looking%20At%20Door? false)
    (Utilities|FlowControl|Gate true
      (:Exit
        (if (Variables|Default|GetIs%20door%20closed?)
          (bind _open_close (Timeline|Timeline_OpenDoor PlayFromStart)
            (:Update
              (Transformation|SetRelativeRotation (Variables|Default|GetSM_Door) (Math|Rotator|MakeRotator 0.0 0.0 (Math|Float|Lerp (Variables|Default|GetOpen%20Angle) (Variables|Default|GetClose%20Angle) _open_close)) false false))
            (:Finished
              (Variables|Default|SetIs%20door%20closed? false)))
          (else
            (bind _open_close_2 (Timeline|Timeline_0 ReverseFromEnd)
              (:Update
                (Transformation|SetRelativeRotation (Variables|Default|GetSM_Door) (Math|Rotator|MakeRotator 0.0 0.0 (Math|Float|Lerp (Variables|Default|GetOpen%20Angle) (Variables|Default|GetClose%20Angle) _open_close_2)) false false))
              (:Finished
                (Variables|Default|SetIs%20door%20closed? true)))))))))

(fn ConstructionScript)