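; Fire hazard prop that repeatedly damages the third-person player character while it stands inside the trigger box.
; Overlap sets OnFire and calls DamageForPlayer, which passes current HP minus a fixed amount to CallOnDamage unless the character is dead.
; A timeline then drives the Damage parameter in MPC_Damage, and its Update loops back through a short Delay until overlap ends or the character dies.
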(event OnComponentBeginOverlap(Box)
  (params (OverlappedComponent :type Primitive%20Component%20Object%20Reference) (OtherActor :type Actor%20Object%20Reference) (OtherComp :type Primitive%20Component%20Object%20Reference) (OtherBodyIndex :type Integer) (bFromSweep :type Boolean) (SweepResult :type Hit%20Result%20Structure%20%28by%20ref%29))
  (Variables|Default|SetOn%20Fire? true)
  (bind _dead_ (CallFunction|DamageforPlayer OtherActor :!label _label))
  (if (not _dead_)
    (bind _newtrack_0 (Timeline|Timeline_0 PlayFromStart)
      (:Update
        (Rendering|Material|SetScalarParameterValue "/Game/Home_Platformer/HUD/MaterialsFromHUD/MPC_Damage.MPC_Damage" "Damage" _newtrack_0 :!class /Script/Engine.KismetMaterialLibrary)
        (if (Variables|Default|GetOn%20Fire?)
          (Utilities|FlowControl|Delay 0.5)
          (goto _label))))))

(event OnComponentEndOverlap(Box)
  (params (OverlappedComponent :type Primitive%20Component%20Object%20Reference) (OtherActor :type Actor%20Object%20Reference) (OtherComp :type Primitive%20Component%20Object%20Reference) (OtherBodyIndex :type Integer))
  (Variables|Default|SetOn%20Fire? false))

(event EventBeginPlay)

(event EventTick
  (params (DeltaSeconds :type Float%20%28single-precision%29)))

(fn ConstructionScript)

(fn DamageforPlayer
  (params (ThirdPersonCharacter :type Actor%20Object%20Reference))
  (bind _asbp_third_person_character (Utilities|Casting|CastToBP_ThirdPersonCharacter ThirdPersonCharacter))
  (if (Variables|/Game/Blueprints/CoreBP/Character/HealthStats.HealthStats_C|GetIs%20Dead? (Variables|/Game/Blueprints/CoreBP/Character/BP_ThirdPersonCharacter.BP_ThirdPersonCharacter_C|GetHealthStats _asbp_third_person_character))
    (return (Variables|/Game/Blueprints/CoreBP/Character/HealthStats.HealthStats_C|GetIs%20Dead? (Variables|/Game/Blueprints/CoreBP/Character/BP_ThirdPersonCharacter.BP_ThirdPersonCharacter_C|GetHealthStats _asbp_third_person_character)))
    (else
      (Default|CallOnDamage _asbp_third_person_character (- (Variables|/Game/Blueprints/CoreBP/Character/HealthStats.HealthStats_C|GetCurrentHP (Variables|/Game/Blueprints/CoreBP/Character/BP_ThirdPersonCharacter.BP_ThirdPersonCharacter_C|GetHealthStats _asbp_third_person_character)) 1e+01)))))