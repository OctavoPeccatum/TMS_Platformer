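; BP_InteractActor is an interactable prop that toggles a spotlight on and off when its Interact event is called.
; A LightOn flag decides whether Interact sets the SpotLight intensity to zero or to full brightness.
; A Box trigger creates and shows an Interact_Promt_Widget when BP_ThirdPersonCharacter overlaps it, and removes that widget when the character leaves.
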(event OnComponentBeginOverlap(Box)
  (params (OverlappedComponent :type Primitive%20Component%20Object%20Reference) (OtherActor :type Actor%20Object%20Reference) (OtherComp :type Primitive%20Component%20Object%20Reference) (OtherBodyIndex :type Integer) (bFromSweep :type Boolean) (SweepResult :type Hit%20Result%20Structure%20%28by%20ref%29))
  (Utilities|Casting|CastToBP_ThirdPersonCharacter OtherActor)
  (bind _returnvalue (UserInterface|CreateWidget "/Game/Home_Platformer/HUD/Widgets/Interact_Promt_Widget.Interact_Promt_Widget_C"))
  (bind _output_get (Variables|Default|SetInteractWidget _returnvalue))
  (UserInterface|Viewport|AddtoViewport _output_get 0))

(event OnComponentEndOverlap(Box)
  (params (OverlappedComponent :type Primitive%20Component%20Object%20Reference) (OtherActor :type Actor%20Object%20Reference) (OtherComp :type Primitive%20Component%20Object%20Reference) (OtherBodyIndex :type Integer))
  (Utilities|Casting|CastToBP_ThirdPersonCharacter OtherActor)
  (Widget|RemovefromParent (Variables|Default|GetInteractWidget)))

(event EventInteract
  (if (Variables|Default|GetLight%20on?)
    (Rendering|Components|Light|SetIntensity (Variables|Default|GetSpotLight) 0.0)
    (Variables|Default|SetLight%20on? false)
    (else
      (Rendering|Components|Light|SetIntensity (Variables|Default|GetSpotLight) 2e+04)
      (Variables|Default|SetLight%20on? true))))

(fn ConstructionScript)