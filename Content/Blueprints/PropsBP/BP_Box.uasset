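; BP_Box is a destructible box prop that turns into a BP_Coin when the player attacks it.
; Tick polls the character and actor references from the Destructible event, requiring IsAttack, InAttackZone and that the referenced death-zone actor is this box.
; On a hit it caches its transform, destroys itself, plays a 2D break sound and spawns the coin at the cached location.
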(event Custom|SpawnActor
  (Game|SpawnActorfromClass "/Game/Blueprints/PropsBP/PickUp/BP_Coin.BP_Coin_C" (Math|Transform|MakeTransform (.location (Variables|Default|GetBoxTransform)) "0, 0, 0" "1,1,1") "AlwaysSpawn" 0 (Game|GetInstigator)))

(event EventDestructible
  (params (As%20BP_ThirPersonCharacter :type BP%20Third%20Person%20Character%20Object%20Reference) (ActorInDeathZone :type Actor%20Object%20Reference)))

(event EventTick
  (params (DeltaSeconds :type Float%20%28single-precision%29))
  (if (Utilities|IsValid (stale EventDestructible As%20BP_ThirPersonCharacter))
    (if (Math|Boolean|ANDBoolean (Variables|/Game/Blueprints/CoreBP/Character/BP_ThirdPersonCharacter.BP_ThirdPersonCharacter_C|GetIsAttack? (stale EventDestructible As%20BP_ThirPersonCharacter)) (Variables|/Game/Blueprints/CoreBP/Character/BP_ThirdPersonCharacter.BP_ThirdPersonCharacter_C|GetInAttackZone? (stale EventDestructible As%20BP_ThirPersonCharacter)) (== (stale EventDestructible ActorInDeathZone) self))
      (Variables|Default|SetBoxTransform (Transformation|GetActorTransform self))
      (Actor|DestroyActor)
      (Audio|PlaySound2D "/Game/Home_Platformer/Sounds/SoundEffect/BoxDestructible_Cue.BoxDestructible_Cue" 1.0 1.0 0.0 0 0)
      (CallFunction|SpawnActor))))

(fn ConstructionScript)