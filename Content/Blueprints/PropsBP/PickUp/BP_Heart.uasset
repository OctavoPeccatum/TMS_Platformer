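; BP_Heart is a heart pickup that grants a heart to the player character when picked up.
; It extends a parent class, forwarding overlap to it and overriding the PickedThisUP event.
; That override runs the parent logic, casts the picking actor to BP_ThirdPersonCharacter, then calls AddAHeart on it, passing itself.
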(event EventBeginPlay
  (|CallParentFunction) ; This node is disabled and will not be called.\nDrag off pins to build functionality.
)

(event Collision|EventActorBeginOverlap
  (params (OtherActor :type Actor%20Object%20Reference))
  (|CallParentFunction OtherActor))

(event EventTick
  (params (DeltaSeconds :type Float%20%28single-precision%29))
  (|CallParentFunction DeltaSeconds) ; This node is disabled and will not be called.\nDrag off pins to build functionality.
)

(event EventPickedThisUP
  (params (ActorPickedThisUp :type Actor%20Object%20Reference))
  (|CallParentFunction 0)
  (bind _asbp_third_person_character (Utilities|Casting|CastToBP_ThirdPersonCharacter ActorPickedThisUp))
  (Default|AddAHeart _asbp_third_person_character self))

(fn ConstructionScript
  (|CallParentFunction))