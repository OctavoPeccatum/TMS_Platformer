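; Checkpoint platform prop that sets the player's respawn point when the third-person character enters its box trigger.
; On overlap it passes the Arrow component's world transform and a self reference to GameplayGM, then turns the platform red to show it is active.
; A ReturnToNormal event restores the metal material and is not called within this Blueprint.
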(event OnComponentBeginOverlap(Box)
  (params (OverlappedComponent :type Primitive%20Component%20Object%20Reference) (OtherActor :type Actor%20Object%20Reference) (OtherComp :type Primitive%20Component%20Object%20Reference) (OtherBodyIndex :type Integer) (bFromSweep :type Boolean) (SweepResult :type Hit%20Result%20Structure%20%28by%20ref%29))
  (Utilities|Casting|CastToBP_ThirdPersonCharacter OtherActor)
  (bind _asgameplay_gm (Utilities|Casting|CastToGameplayGM (Game|GetGameMode)))
  (Default|UpdateRespawnPoint _asgameplay_gm (Transformation|GetWorldTransform (Variables|Default|GetArrow)) self)
  (Rendering|Material|SetMaterial (Variables|Default|GetSM_CheckpointPlatform) 0 "/Game/Home_Platformer/Props/Red.Red"))

(event Custom|ReturnToNormal
  (Rendering|Material|SetMaterial (Variables|Default|GetSM_CheckpointPlatform) 0 "/Game/Home_Platformer/Props/Level2/Metal.Metal"))

(event EventBeginPlay)

(event Collision|EventActorBeginOverlap
  (params (OtherActor :type Actor%20Object%20Reference)))

(event EventTick
  (params (DeltaSeconds :type Float%20%28single-precision%29)))

(fn ConstructionScript)