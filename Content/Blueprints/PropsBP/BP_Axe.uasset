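; BP_Axe is a collectible axe pickup that spins and bobs in place until a player character touches it.
; Tick calls AxesJumpAndRotate, which adds a fixed rotation each frame and a local Z offset from the sine of a time-accumulated, wrapped angle.
; Overlapping its Sphere casts the other actor to BP_ThirdPersonCharacter and passes the axe to that character's FCollectedAxe, which handles the collection.
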(event OnComponentBeginOverlap(Sphere)
  (params (OverlappedComponent :type Primitive%20Component%20Object%20Reference) (OtherActor :type Actor%20Object%20Reference) (OtherComp :type Primitive%20Component%20Object%20Reference) (OtherBodyIndex :type Integer) (bFromSweep :type Boolean) (SweepResult :type Hit%20Result%20Structure%20%28by%20ref%29))
  (bind _asbp_third_person_character (Utilities|Casting|CastToBP_ThirdPersonCharacter OtherActor))
  (Default|FCollectedAxe _asbp_third_person_character self))

(event EventTick
  (params (DeltaSeconds :type Float%20%28single-precision%29))
  (CallFunction|AxesJumpandRotate DeltaSeconds))

(fn ConstructionScript)

(fn AxesJumpandRotate
  (params (Delta :type Float%20%28single-precision%29))
  (bind _output_get (Variables|Default|SetSin (Math|Float|%(Float) (+ (* Delta 1e+02) (Variables|Default|GetSin)) 3.6e+02)))
  (Transformation|AddActorLocalRotation "0,5.000000, 0" false false)
  (Transformation|AddActorLocalOffset (Math|Vector|MakeVector 0.0 0.0 (Math|Trig|Sin(Degrees) _output_get)) false false))