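; Pig AI pawn for the platformer that runs away when the third-person player character enters its sphere.
; Sphere overlap events toggle IsNear, and entering triggers the RunAway event.
; RunAway projects a point directly away from the player, picks a random reachable location around it and moves there with AI MoveTo.
; Each successful move calls RunAway again with IsNear, chaining escapes without using Tick.
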(event OnComponentBeginOverlap(Sphere)
  (params (OverlappedComponent :type Primitive%20Component%20Object%20Reference) (OtherActor :type Actor%20Object%20Reference) (OtherComp :type Primitive%20Component%20Object%20Reference) (OtherBodyIndex :type Integer) (bFromSweep :type Boolean) (SweepResult :type Hit%20Result%20Structure%20%28by%20ref%29))
  (if (== OtherActor (Variables|Default|GetAs%20BP%20Third%20Person%20Character))
    (bind _output_get (Variables|Default|SetIs%20Near? true))
    (CallFunction|RunAway _output_get)))

(event OnComponentEndOverlap(Sphere)
  (params (OverlappedComponent :type Primitive%20Component%20Object%20Reference) (OtherActor :type Actor%20Object%20Reference) (OtherComp :type Primitive%20Component%20Object%20Reference) (OtherBodyIndex :type Integer))
  (if (== OtherActor (Variables|Default|GetAs%20BP%20Third%20Person%20Character))
    (Variables|Default|SetIs%20Near? false)))

(event Custom|RunAway
  (params (IsNear? :type Boolean))
  (bind _returnvalue (Transformation|GetActorLocation))
  (bind _as_bp_third_person_character (Variables|Default|GetAs%20BP%20Third%20Person%20Character))
  (bind _returnvalue_2 (Transformation|GetActorLocation _as_bp_third_person_character))
  (bind _returnvalue_3 (Math|Rotator|FindLookatRotation _returnvalue _returnvalue_2))
  (bind _returnvalue_4 (Math|Vector|GetForwardVector _returnvalue_3))
  (bind _returnvalue_5 (* _returnvalue_4 -5e+02))
  (bind _returnvalue_6 (+ _returnvalue _returnvalue_5))
  (bind (_x _y) (Math|Vector|BreakVector _returnvalue_6))
  (if IsNear?
    (AI|AIMoveTo self (.RandomLocation (AI|Navigation|GetRandomReachablePointinRadius (Math|Vector|MakeVector _x _y (.Z (Math|Vector|BreakVector _returnvalue))) 5e+02 0 0)) 0 5.0 false
      (:OnSuccess
        (CallFunction|RunAway (Variables|Default|GetIs%20Near?))))))

(event EventBeginPlay
  (bind _asbp_third_person_character (Utilities|Casting|CastToBP_ThirdPersonCharacter (Game|GetPlayerCharacter 0)))
  (Variables|Default|SetAs%20BP%20Third%20Person%20Character _asbp_third_person_character))

(fn ConstructionScript)