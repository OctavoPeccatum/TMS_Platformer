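; Player controller that owns the main HUD and opens the escape and next-level menus.
; BeginPlay creates the HUD and intro sound; the EscapeMenu input and WinGame event each spawn their menu.
; Both menu rule functions hide the HUD, pause, show the cursor, play the sound and set UI-only input, both focusing the EscapeMenu widget.
; CloseEscapeMenu clears that menu's reference and restores HUD, game input and play.
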(event Custom|WinGame
  (bind _returnvalue (UserInterface|CreateWidget "/Game/Home_Platformer/HUD/Widgets/W_NextLevelMenu.W_NextLevelMenu_C" self))
  (bind _output_get (Variables|Default|SetNextLevel _returnvalue))
  (UserInterface|Viewport|AddtoViewport _output_get 0)
  (CallFunction|NextLevelMenuRules))

(event EventBeginPlay
  (bind _returnvalue (UserInterface|CreateWidget "/Game/Home_Platformer/HUD/Widgets/MainHUD.MainHUD_C" self))
  (bind _output_get (Variables|Default|SetMain%20HUD _returnvalue))
  (UserInterface|Viewport|AddtoViewport _output_get 0)
  (bind _returnvalue_2 (Audio|CreateSound2D "/Game/Home_Platformer/Sounds/MusicSound/S_MenuIntro.S_MenuIntro" 1.0 1.0 0.0 0))
  (Variables|Default|SetMenuIntroSound _returnvalue_2))

(event EventTick
  (params (DeltaSeconds :type Float%20%28single-precision%29)))

(event Input|ActionEvents|InputActionEscapeMenu
  (params (Key :type Key%20Structure :default "None"))
  (:Pressed
    (bind _returnvalue (UserInterface|CreateWidget "/Game/Home_Platformer/HUD/Widgets/W_EscapeMenu.W_EscapeMenu_C" self))
    (bind _output_get (Variables|Default|SetEscapeMenu _returnvalue))
    (UserInterface|Viewport|AddtoViewport _output_get 0)
    (CallFunction|EscapeMenuRules)))

(fn ConstructionScript)

(fn CloseEscapeMenu
  (Variables|Default|SetEscapeMenu 0)
  (Widget|SetVisibility (Variables|Default|GetMain%20HUD) "Visible")
  (Input|SetInputModeGameOnly self)
  (Variables|Default|SetbShowMouseCursor false)
  (Game|SetGamePaused false))

(fn EscapeMenuRules
  (Widget|SetVisibility (Variables|Default|GetMain%20HUD) "Hidden")
  (Input|SetInputModeUIOnly self (Variables|Default|GetEscapeMenu) "DoNotLock")
  (Variables|Default|SetbShowMouseCursor true)
  (Game|SetGamePaused true)
  (Audio|Components|Audio|Play (Variables|Default|GetMenuIntroSound) 0.0))

(fn NextLevelMenuRules
  (Widget|SetVisibility (Variables|Default|GetMain%20HUD) "Hidden")
  (Input|SetInputModeUIOnly self (Variables|Default|GetEscapeMenu) "DoNotLock")
  (Variables|Default|SetbShowMouseCursor true)
  (Game|SetGamePaused true)
  (Audio|Components|Audio|Play (Variables|Default|GetMenuIntroSound) 0.0))