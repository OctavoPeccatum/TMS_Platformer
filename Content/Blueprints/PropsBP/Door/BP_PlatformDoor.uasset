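; BP_PlatformDoor is a colored, key-locked door that fades out and becomes passable when a player with a matching key reaches it.
; BeginPlay creates dynamic materials for three mesh slots and applies DoorColor to the first.
; Overlapping DoorInteractZone checks the character's KeysCollected against the DoorType tag query, then opens the door and deletes the key.
; Opening runs once, disabling collision, playing a sound and driving all three materials' Opacity through a timeline.
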(event OnComponentBeginOverlap(DoorInteractZone)
  (params (OverlappedComponent :type Primitive%20Component%20Object%20Reference) (OtherActor :type Actor%20Object%20Reference) (OtherComp :type Primitive%20Component%20Object%20Reference) (OtherBodyIndex :type Integer) (bFromSweep :type Boolean) (SweepResult :type Hit%20Result%20Structure%20%28by%20ref%29))
  (bind _asbp_third_person_character (Utilities|Casting|CastToBP_ThirdPersonCharacter OtherActor))
  (if (GameplayTags|DoesContainerMatchTagQuery (Variables|/Game/Blueprints/CoreBP/Character/BP_ThirdPersonCharacter.BP_ThirdPersonCharacter_C|GetKeysCollected _asbp_third_person_character) (Variables|Default|GetDoorType))
    (CallFunction|OpentheGate)
    (Default|DeleteKey _asbp_third_person_character)))

(event Custom|OpenTheGate
  (Utilities|FlowControl|DoOnce false
    (:Completed
      (Collision|SetCollisionEnabled (Variables|Default|GetSM_Door) "NoCollision")
      (Audio|SpawnSound2D "/Game/Home_Platformer/Sounds/MusicSound/opendoor.opendoor" 1.0 1.0 0.0 0)
      (bind _dooropasity (Timeline|T_Door Play)
        (:Update
          (Utilities|FlowControl|Sequence
            (:then_0
              (Rendering|Material|SetScalarParameterValue (Variables|Default|GetDoorDynamicMaterial) "Opacity" _dooropasity :!class /Script/Engine.MaterialInstanceDynamic))
            (:then_1
              (Rendering|Material|SetScalarParameterValue (Variables|Default|GetDoorDynamicMaterial2) "Opacity" _dooropasity :!class /Script/Engine.MaterialInstanceDynamic))
            (:then_2
              (Rendering|Material|SetScalarParameterValue (Variables|Default|GetDoorDunamicMaterial3) "Opacity" _dooropasity :!class /Script/Engine.MaterialInstanceDynamic))))))))

(event EventBeginPlay
  (bind _returnvalue (Rendering|Material|CreateDynamicMaterialInstance (Variables|Default|GetSM_Door) 0 "/Game/Home_Platformer/Props/Home2/VilagePropsPackLite/Models/MI_19_Default.MI_19_Default" "None" :!class /Script/Engine.PrimitiveComponent))
  (bind _output_get (Variables|Default|SetDoorDynamicMaterial _returnvalue))
  (bind _returnvalue_2 (Rendering|Material|CreateDynamicMaterialInstance (Variables|Default|GetSM_Door) 1 "/Game/Home_Platformer/Props/Level2/MI_Wood.MI_Wood" "None" :!class /Script/Engine.PrimitiveComponent))
  (Variables|Default|SetDoorDynamicMaterial2 _returnvalue_2)
  (bind _returnvalue_3 (Rendering|Material|CreateDynamicMaterialInstance (Variables|Default|GetSM_Door) 2 "/Game/Home_Platformer/Props/Level2/MI_Wood_Light.MI_Wood_Light" "None" :!class /Script/Engine.PrimitiveComponent))
  (Variables|Default|SetDoorDunamicMaterial3 _returnvalue_3)
  (Rendering|Material|SetVectorParameterValue _output_get "ColorDoor" (Variables|Default|GetDoorColor) :!class /Script/Engine.MaterialInstanceDynamic))

(fn ConstructionScript)